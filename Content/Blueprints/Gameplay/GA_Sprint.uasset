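; Gameplay Ability that makes a CoreCharacterBasic avatar sprint while active.
; Activation ends immediately if the avatar is stationary or the cost commit fails; only cost is committed, not cooldown.
; On success it raises MaxWalkSpeed to RunSpeed and waits for the Movement.StopRun gameplay event to end.
; OnEndAbility restores WalkSpeed; the GetMaxSpeed helper is unused in this graph.
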(event `self.K2_ActivateAbility`
  (if (not (`KismetMathLibrary.Vector_IsZero` (`self.GetVelocity`)))
    (bind _returnvalue (`self.K2_CommitAbilityCost` false))
    (if _returnvalue
      (bind _ascore_character_basic (cast `CoreCharacterBasic` (`self.GetAvatarActorFromActorInfo`)))
      (`/Engine/EditorBlueprintResources/StandardMacros.IsValid` _ascore_character_basic
        (:`Is Valid`
          (set `CharacterMovementComponent.MaxWalkSpeed` (`CoreCharacterBasic.RunSpeed` _ascore_character_basic) (`Character.CharacterMovement` _ascore_character_basic))
          (`AbilityTask_WaitGameplayEvent.WaitGameplayEvent` (struct :`TagName` "Gameplay.Events.Movement.StopRun") null
            (:`EventReceived`
              (`self.K2_EndAbility`))))
        (:`Is Not Valid`
          (`self.K2_EndAbility` :!label _label)))
      (else
        (goto _label)))
    (else
      (goto _label))))

(event `self.K2_OnEndAbility`
  (params (bWasCancelled :type Boolean))
  (bind _ascore_character_basic (cast `CoreCharacterBasic` (`self.GetAvatarActorFromActorInfo`)))
  (`/Engine/EditorBlueprintResources/StandardMacros.IsValid` _ascore_character_basic
    (:`Is Valid`
      (set `CharacterMovementComponent.MaxWalkSpeed` (`CoreCharacterBasic.WalkSpeed` _ascore_character_basic) (`Character.CharacterMovement` _ascore_character_basic)))))

(fn `GetMaxSpeed`
  (returns (ReturnValue :type "Float (double-precision)"))
  (bind _aspawn (cast `Pawn` (`self.GetAvatarActorFromActorInfo`)))
  (return (`MovementComponent.GetMaxSpeed` (`Pawn.GetMovementComponent` _aspawn))))

(fn `GetVelocity`
  (returns (ReturnValue :type "Vector Structure"))
  (bind _aspawn (cast `Pawn` (`self.GetAvatarActorFromActorInfo`)))
  (return (`Actor.GetVelocity` _aspawn)))