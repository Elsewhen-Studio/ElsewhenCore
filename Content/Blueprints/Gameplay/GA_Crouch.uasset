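; Gameplay ability that makes the BP_CharacterBasic avatar crouch.
; On activation it calls BeginCrouch on the character and waits for the StopCrouch movement gameplay event.
; When that event arrives, a very short delay precedes EndCrouch and the end of the ability.
; A TimelineMacro with optional cosine easing and looping is also defined, but the ability's event graph does not use it.
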(event `self.K2_ActivateAbility`
  (`|ExecutionSequence`
    (:`then_0`
      (bind _asbp_character_basic (cast `/ElsewhenCore/Blueprints/BP_CharacterBasic` (`self.GetAvatarActorFromActorInfo`)))
      (`/ElsewhenCore/Blueprints/BP_CharacterBasic.BeginCrouch` _asbp_character_basic))
    (:`then_1`
      (`AbilityTask_WaitGameplayEvent.WaitGameplayEvent` (struct :`TagName` "Gameplay.Events.Movement.StopCrouch") null
        (:`EventReceived`
          (`AbilityTask_WaitDelay.WaitDelay` 0.025
            (:`then`
              (bind _asbp_character_basic_2 (cast `/ElsewhenCore/Blueprints/BP_CharacterBasic` (`self.GetAvatarActorFromActorInfo`)))
              (`/ElsewhenCore/Blueprints/BP_CharacterBasic.EndCrouch` _asbp_character_basic_2)
              (`self.K2_EndAbility`))))))))

(event `self.K2_OnEndAbility`
  (params (bWasCancelled :type Boolean)))