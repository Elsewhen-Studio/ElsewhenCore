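; Player character Blueprint that handles sprint energy through the Gameplay Ability System and adds procedural camera headbob.
; Energy loss cancels regen and reapplies an effect after a delay; full energy removes regen, and empty energy stops sprinting via gameplay event and tag-based effect removal.
; Landing sends a gameplay event.
; Headbob smoothly interpolates speed-scaled sine waves into camera height, roll and idle pitch sway, advancing the bob timer only while grounded.
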(event `HandleEnergy`
  (params (NewValue :type "Float (double-precision)") (OldValue :type "Float (double-precision)"))
  (bind (_maxenergy_basevalue _maxenergy_currentvalue) (break `GameplayAttributeData` (`BasicAttributes.MaxEnergy` (`self.BasicAttributes`))))
  (`|ExecutionSequence`
    (:`then_0`
      (if (< NewValue OldValue)
        (`AbilitySystemComponent.RemoveActiveEffectsWithGrantedTags` (`self.ASC`) (struct :`GameplayTags` (struct :`(TagName` "Gameplay.Status.Energy.Regen"))))
        (`KismetSystemLibrary.Delay` 5.0)
        (`AbilitySystemComponent.BP_ApplyGameplayEffectToSelf` :`self` (`self.ASC`))
        (elif (>= NewValue _maxenergy_currentvalue)
          (`AbilitySystemComponent.RemoveActiveEffectsWithGrantedTags` (`self.ASC`) (struct :`GameplayTags` (struct :`(TagName` "Gameplay.Status.Energy.Regen")))))))
    (:`then_1`
      (if (<= NewValue 0.0)
        (`self.StopSprinting`)))))

(event `self.ReceiveBeginPlay`
  (`|ExecutionSequence`
    (:`then_0`
      (set `self.BaseCamLoc` (`SceneComponent.RelativeLocation` (`self.CameraComponent`))))))

(event `self.OnLanded`
  (params (Hit :type "HitResult Structure (by ref)"))
  (`AbilitySystemBlueprintLibrary.SendGameplayEventToActor` self (struct :`TagName` "Gameplay.Events.Movement.Landed")))

(event `Headbob`
  (bind _runspeed (`self.RunSpeed`))
  (bind _cameracomponent (`self.CameraComponent`))
  (bind _returnvalue (`KismetMathLibrary.VSize` (`self.GetVelocity`)))
  (bind _returnvalue_2 (`KismetMathLibrary.MapRangeClamped` _returnvalue 0.0 _runspeed 0.0 1.0))
  (bind _returnvalue_3 (* (`KismetMathLibrary.Lerp` (`self.WalkBobRoll`) (`self.SprintBobRoll`) _returnvalue_2) _returnvalue_2))
  (if (and (`self.CanJump`) (`NavMovementComponent.IsMovingOnGround` (`self.CharacterMovement`)))
    (set `self.BobTimer` (+ (`self.BobTimer`) (* (`GameplayStatics.GetWorldDeltaSeconds`) (`KismetMathLibrary.Lerp` (`self.WalkFrequency`) (`self.SprintFrequency`) (`KismetMathLibrary.MapRangeClamped` _returnvalue 0.0 _runspeed 0.0 1.0)))))
    (else
      (set `self.BobTimer` 0.0)))
  (`SceneComponent.K2_SetRelativeLocation` _cameracomponent (`KismetMathLibrary.VInterpTo` (`SceneComponent.RelativeLocation` (`self.CameraComponent`)) (+ (`KismetMathLibrary.MakeVector` 0.0 0.0 (* (* (`KismetMathLibrary.Sin` (`self.BobTimer`)) _returnvalue_3) (`self.BobHeight`))) (`self.BaseCamLoc`)) (`GameplayStatics.GetWorldDeltaSeconds`) (`self.InterpSpeed`)) false false)
  (`SceneComponent.K2_SetRelativeRotation` _cameracomponent (`KismetMathLibrary.RInterpTo` (`SceneComponent.RelativeRotation` (`self.CameraComponent`)) (`KismetMathLibrary.MakeRotator` (* (* _returnvalue_3 (`KismetMathLibrary.Sin` (* (`self.BobTimer`) 0.5))) (`self.BobRoll`)) (* (* (`KismetMathLibrary.Sin` (* (`self.IdleTimer`) 2.0)) (`self.IdlePitch`)) (`KismetMathLibrary.MapRangeClamped` _returnvalue 0.0 (`self.WalkSpeed`) 1.0))) (`GameplayStatics.GetWorldDeltaSeconds`) (`self.InterpSpeed`)) false false :!label _label))

(event `HeadbobIdle`
  (set `self.IdleTimer` (+ (`GameplayStatics.GetWorldDeltaSeconds`) (`self.IdleTimer`)))
  (goto _label))

(fn `StopSprinting`
  (`AbilitySystemBlueprintLibrary.SendGameplayEventToActor` self (struct :`TagName` "Gameplay.Events.Movement.StopRun"))
  (`AbilitySystemComponent.RemoveActiveEffectsWithGrantedTags` (`self.ASC`) (struct :`GameplayTags` (struct :`(TagName` "Gameplay.Status.Energy.Consume")))))

(fn `UserConstructionScript`)